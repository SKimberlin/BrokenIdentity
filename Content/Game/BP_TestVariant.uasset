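; BP_TestVariant is a test Blueprint that prototypes a light/heavy attack combo check, reporting results only through Print String.
; AttemptCombo switches on the integer CurrentCombo and branches on AttackType, storing the opening attack and resetting after the second.
; Recognized pairs are Light-Light, Light-Heavy and Heavy-Heavy, while Heavy-Light prints as no combo.
; States 2, 3 and 5 are never assigned here, and the event graph holds only disabled default events.
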(fn `AttemptCombo`
  (params (AttackType :type "/Game/Game/E_AttackType Enum" :default "NewEnumerator0"))
  (bind _returnvalue (`|EnumEquality` AttackType "NewEnumerator0"))
  (switch `int` (`self.CurrentCombo`)
    (:`0`
      (if _returnvalue
        (set `self.CurrentCombo` 1)
        (`KismetSystemLibrary.PrintString` "Light")
        (else
          (set `self.CurrentCombo` 4)
          (`KismetSystemLibrary.PrintString` "Heavy"))))
    (:`1`
      (if _returnvalue
        (set `self.CurrentCombo` 0)
        (`KismetSystemLibrary.PrintString` "Light, Light")
        (else
          (set `self.CurrentCombo` 0)
          (`KismetSystemLibrary.PrintString` "Light, Heavy"))))
    (:`2`
      (if _returnvalue
        (set `self.CurrentCombo` 0)
        (`KismetSystemLibrary.PrintString` "Not Combo")))
    (:`3`
      (if _returnvalue
        (set `self.CurrentCombo` 0)
        (`KismetSystemLibrary.PrintString` "Not Combo")))
    (:`4`
      (if _returnvalue
        (set `self.CurrentCombo` 0)
        (`KismetSystemLibrary.PrintString` "Not Combo")
        (else
          (set `self.CurrentCombo` 0)
          (`KismetSystemLibrary.PrintString` "Heavy, Heavy"))))
    (:`5`
      (if _returnvalue
        (set `self.CurrentCombo` 0)
        (`KismetSystemLibrary.PrintString` "Not Combo")))))

(fn `UserConstructionScript`
  (`parent.UserConstructionScript`))