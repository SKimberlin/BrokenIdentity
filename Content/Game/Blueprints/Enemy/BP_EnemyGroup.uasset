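; BP_EnemyGroup tracks a group of enemies through a Members array and a Leader reference.
; AddToGroup appends an enemy only when Find already locates it in Members, so the check appears inverted and new enemies are never added through it.
; NewLeader promotes the first member not flagged Dead and leaves Leader unchanged when none qualifies.
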(fn `AddToGroup`
  (params (NewMember :type "/Game/Game/Blueprints/Enemy/BP_Enemy Object Reference"))
  (bind _members (`self.Members`))
  (if (!= (`KismetArrayLibrary.Array_Find` _members NewMember) -1)
    (`KismetArrayLibrary.Array_Add` _members NewMember)))

(fn `NewLeader`
  (for _array_element (`self.Members`)
    (if (not (`/Game/Game/Blueprints/Enemy/BP_Enemy.Dead` _array_element))
      (set `self.Leader` _array_element)
      (break))))