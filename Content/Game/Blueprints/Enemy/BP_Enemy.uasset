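; BP_Enemy is a melee enemy character with a world-space health bar and group alerting that shares targets with member AI controllers.
; Attacks reserve tokens from the player, play a punch montage and return them when it ends, with a hand sphere trace applying damage.
; Damage updates health and triggers a hit reaction through the AI controller.
; Death stops AI logic and, looping over reserved tokens, returns them and ragdolls the body.
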(event `self.ReceiveBeginPlay`
  (bind _characterstatcomponent (`self.CharacterStatComponent`))
  (bind _aswbp_world_health_bar (cast `/Game/Game/Blueprints/Widgets/WBP_WorldHealthBar` (`WidgetComponent.GetWidget` (`self.HealthBar`))))
  (bind _output_get (set `self.HealthBarWidget` _aswbp_world_health_bar))
  (set `/Game/Game/Blueprints/Widgets/WBP_WorldHealthBar.HealthPercent` (/ (`/Game/Game/CharacterStatComponent.Health` _characterstatcomponent) (`/Game/Game/CharacterStatComponent.MaxHealth` _characterstatcomponent)) _output_get))

(event `self.ReceiveTick`
  (params (DeltaSeconds :type "Float (single-precision)")))

(event `self.ReceiveAnyDamage`
  (params (Damage :type "Float (single-precision)") (DamageType :type "DamageType Object Reference") (InstigatedBy :type "Controller Object Reference") (DamageCauser :type "Actor Object Reference"))
  (bind _aicontroller (`self.AIController`))
  (bind _reservedtokens (`self.ReservedTokens`))
  (bind _characterstatcomponent (`self.CharacterStatComponent`))
  (bind _mesh (`self.Mesh`))
  (bind _characterstatcomponent_2 (`self.CharacterStatComponent`))
  (bind _output_get (set `/Game/Game/CharacterStatComponent.Health` (- (`/Game/Game/CharacterStatComponent.Health` _characterstatcomponent) Damage) _characterstatcomponent))
  (bind _returnvalue (<= _output_get 0.0))
  (if _returnvalue
    (set `self.Dead` _returnvalue)
    (`BrainComponent.StopLogic` (`AIController.BrainComponent` (`AIBlueprintHelperLibrary.GetAIController` self)) "Dead")
    (bind _keys (`BlueprintMapLibrary.Map_Keys` _reservedtokens))
    (for _array_element _keys
      (bind _asbp_base_player (cast `/Game/Game/Blueprints/Characters/BP_BasePlayer` _array_element))
      (`/Game/Game/Blueprints/Characters/BP_BasePlayer.ReturnToken` _asbp_base_player (`BlueprintMapLibrary.Map_Find` _reservedtokens _array_element))
      (`PrimitiveComponent.SetSimulatePhysics` _mesh true)
      (`CharacterMovementComponent.DisableMovement` (`self.CharacterMovement`))
      (`PrimitiveComponent.SetCollisionProfileName` _mesh "Ragdoll" true)
      (`SceneComponent.SetVisibility` (`self.HealthBar`) false false)
      (`PrimitiveComponent.SetCollisionEnabled` (`self.CapsuleComponent`) "NoCollision"))
    (else
      (set `/Game/Game/Blueprints/Widgets/WBP_WorldHealthBar.HealthPercent` (/ (`/Game/Game/CharacterStatComponent.Health` _characterstatcomponent_2) (`/Game/Game/CharacterStatComponent.MaxHealth` _characterstatcomponent_2)) (`self.HealthBarWidget`))
      (`|PlayMontage` (`self.Mesh`) "/Game/Game/Animations/FullMelee/Hit_Reaction_Montage.Hit_Reaction_Montage"
        (:`then`
          (`/Game/Game/Blueprints/Enemy/AIC_Enemy.Hit` _aicontroller DamageCauser))
        (:`OnCompleted`
          (`/Game/Game/Blueprints/Enemy/AIC_Enemy.SetBlackboardState` _aicontroller "NewEnumerator1" :!label _label))
        (:`OnInterrupted`
          (goto _label))))))

(event `Attack`
  (params (Target :type "Actor Object Reference"))
  (set `self.Attacking` true)
  (`|PlayMontage` (`self.Mesh`) "/Game/Game/Animations/FullMelee/Attacks/Punches/Punching__1__Montage.Punching__1__Montage"
    (:`OnCompleted`
      _)
    (:`OnInterrupted`
      _))
  (`self.AttackEnd` Target))

(fn `AlertGroup`
  (params (Target :type "Actor Object Reference"))
  (bind _group_members (break `/Game/Game/Blueprints/Enemy/S_EnemyGroup` (`self.Group`)))
  (for _array_element _group_members
    (`/Game/Game/Blueprints/Enemy/AIC_Enemy.SetTarget` (`/Game/Game/Blueprints/Enemy/BP_Enemy.AIController` _array_element) Target)))

(fn `AttackEnd`
  (params (Target :type "Actor Object Reference"))
  (bind _currentheldtokens (`self.CurrentHeldTokens`))
  (bind _asbp_base_player (cast `/Game/Game/Blueprints/Characters/BP_BasePlayer` Target))
  (`/Game/Game/Blueprints/Characters/BP_BasePlayer.ReturnToken` _asbp_base_player _currentheldtokens)
  (bind _result (`/Engine/EditorBlueprintResources/StandardMacros.NegateInt` _currentheldtokens)
    (:`  `
      (`self.StoreAttackTokens` _asbp_base_player _result)
      (set `self.Attacking` false))))

(fn `AttackStart`
  (params (Target :type "Actor Object Reference") (Tokens :type Integer))
  (returns (Success :type Boolean))
  (bind _asbp_base_player (cast `/Game/Game/Blueprints/Characters/BP_BasePlayer` Target))
  (bind _recievetoken (`/Game/Game/Blueprints/Characters/BP_BasePlayer.RequestToken` _asbp_base_player Tokens))
  (if _recievetoken
    (`self.StoreAttackTokens` _asbp_base_player Tokens)
    (set `self.CurrentHeldTokens` Tokens)
    (return true)
    (else
      (return false))))

(fn `HealthBarVisibility`
  (params (Visible :type Boolean))
  (`SceneComponent.SetVisibility` (`self.HealthBar`) Visible false))

(fn `HitDetect`
  (bind _returnvalue (`SceneComponent.GetSocketLocation` (`self.Mesh`) "hand_r"))
  (if (not (`self.HitTarget`))
    (bind _outhit (`KismetSystemLibrary.SphereTraceSingleForObjects` :`Start` _returnvalue :`End` _returnvalue :`Radius` 75.0 :`ObjectTypes` (`|MakeArray` "ObjectTypeQuery3" :!type "EObjectTypeQuery Enum") :`DrawDebugType` "ForDuration"))
    (bind _asbp_base_player (cast `/Game/Game/Blueprints/Characters/BP_BasePlayer` (`.HitActor` (`GameplayStatics.BreakHitResult` _outhit))))
    (`GameplayStatics.ApplyDamage` _asbp_base_player 10.0 null null "/Script/Engine.DamageType")
    (set `self.HitTarget` true)))

(fn `SetMovementSpeed`
  (params (Speed :type "Float (double-precision)"))
  (set `CharacterMovementComponent.MaxWalkSpeed` Speed (`self.CharacterMovement`)))

(fn `StoreAttackTokens`
  (params (Target :type "Actor Object Reference") (Amount :type Integer))
  (bind (_value _returnvalue) (`BlueprintMapLibrary.Map_Find` (`self.ReservedTokens`) Target))
  (`BlueprintMapLibrary.Map_Add` (`self.ReservedTokens`) Target (`KismetMathLibrary.SelectInt` (+ Amount _value) Amount _returnvalue)))

(fn `UserConstructionScript`
  (set `self.Group` (make `/Game/Game/Blueprints/Enemy/S_EnemyGroup` _ 0 self)))