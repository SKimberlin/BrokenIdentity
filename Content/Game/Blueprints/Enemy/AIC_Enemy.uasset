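; AIC_Enemy is the enemy AI controller, which runs the BT_Enemy behavior tree on possess and on BeginPlay.
; When perception updates on a BP_BasePlayer, it stores that player as the blackboard target and switches the enemy state, without checking whether the stimulus was gained or lost.
; A forgotten-target event sets the other state but leaves the target set.
; SetLeader writes a leader actor into the blackboard.
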(event `self.ReceivePossess`
  (params (PossessedPawn :type "Pawn Object Reference"))
  (`self.RunBehaviorTree` "/Game/Game/Blueprints/Enemy/BT_Enemy.BT_Enemy" :!label _label))

(event `self.ReceiveBeginPlay`
  (goto _label))

(event `self.AIPerception.OnTargetPerceptionUpdated`
  (params (Actor :type "Actor Object Reference") (Stimulus :type "AIStimulus Structure"))
  (bind _returnvalue (`AIBlueprintHelperLibrary.GetBlackboard` null))
  (bind _asbp_base_player (cast `/Game/Game/Blueprints/Characters/BP_BasePlayer` Actor))
  (set `self.Target` _asbp_base_player)
  (`BlackboardComponent.SetValueAsObject` _returnvalue (`self.TargetKey`) _asbp_base_player)
  (`BlackboardComponent.SetValueAsEnum` _returnvalue (`self.StateKey`) (enumliteral `/Game/Game/Blueprints/Enemy/E_EnemyState` "NewEnumerator1")))

(event `self.AIPerception.OnTargetPerceptionForgotten`
  (params (Actor :type "Actor Object Reference"))
  (`BlackboardComponent.SetValueAsEnum` (`AIBlueprintHelperLibrary.GetBlackboard` null) (`self.StateKey`) (enumliteral `/Game/Game/Blueprints/Enemy/E_EnemyState` "NewEnumerator0")))

(fn `SetLeader`
  (params (Leader :type "/Game/Game/Blueprints/Enemy/BP_Enemy Object Reference"))
  (locals (LeaderKey :type Name :default "Leader"))
  (`BlackboardComponent.SetValueAsObject` (`AIBlueprintHelperLibrary.GetBlackboard` null) (`local.LeaderKey`) Leader))

(fn `UserConstructionScript`)