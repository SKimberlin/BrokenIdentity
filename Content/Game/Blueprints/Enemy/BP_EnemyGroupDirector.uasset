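; Director actor that periodically spawns groups of BP_Enemy around the player, up to a maximum group count.
; A looping one-second timer rolls a spawn chance, then tests one random reachable point for minimum distance from the player and each group's first member.
; Enemies scatter around that point and share a group struct holding members, an unused ID and the first member.
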(event `self.ReceiveBeginPlay`
  (`KismetSystemLibrary.K2_SetTimerDelegate` (delegate `TrySpawnGroup`) 1.0 true))

(event `self.ReceiveTick`
  (params (DeltaSeconds :type "Float (single-precision)")))

(event `TrySpawnGroup`
  (if (`self.SpawningActive`)
    (if (< (`KismetArrayLibrary.Array_Length` (`self.Groups`)) (`self.MaxGroups`))
      (if (<= (`KismetMathLibrary.RandomFloat`) (`self.SpawnChance`))
        (`self.SpawnGroup`)))))

(fn `GetSpawnPoint`
  (returns (Location :type "Vector Structure") (FoundLocation :type Boolean))
  (locals (PlayerLocation :type "Vector Structure") (MaxDistance :type "Float (double-precision)" :default 50000.0) (MinDistance :type "Float (double-precision)" :default 1000.0) (ReturnLocation :type "Vector Structure") (ValidLocation :type Boolean :default true))
  (bind _output_get (set `local.PlayerLocation` (`self.K2_GetActorLocation` (`GameplayStatics.GetPlayerCharacter` 0))))
  (bind _output_get_2 (set `local.ReturnLocation` (`NavigationSystemV1.K2_GetRandomReachablePointInRadius` _output_get (`local.MaxDistance`) null null)))
  (if (>= (`KismetMathLibrary.VSizeXY` (- (`local.PlayerLocation`) _output_get_2)) (`local.MinDistance`))
    (for _array_element (`self.Groups`)
      (if (not (>= (`KismetMathLibrary.VSizeXY` (- (`self.K2_GetActorLocation` (`|GetArrayItem` (break `/Game/Game/Blueprints/Enemy/S_EnemyGroup` _array_element))) _output_get_2)) (`local.MinDistance`)))
        (set `local.ValidLocation` false)
        (break)))
    (return (`local.ReturnLocation`) (`local.ValidLocation`))
    (else
      (return (`local.ReturnLocation`) false))))

(fn `GetUnusedID`
  (returns (ID :type Integer))
  (locals (FreeID :type Integer))
  (bind _freeid (`local.FreeID`))
  (for _index (range (+ (`self.MaxGroups`) 1))
    (if (not (`KismetArrayLibrary.Array_Contains` (`self.UsedIDs`) _index))
      (set `local.FreeID` _index)
      (break)))
  (`KismetArrayLibrary.Array_Add` (`self.UsedIDs`) _freeid)
  (return _freeid))

(fn `SpawnGroup`
  (locals (MainSpawnPoint :type "Vector Structure") (NotSpawned :type Boolean) (CurrentGroup :type "/Game/Game/Blueprints/Enemy/S_EnemyGroup Structure"))
  (bind (_currentgroup_members _currentgroup_id) (break `/Game/Game/Blueprints/Enemy/S_EnemyGroup` (`local.CurrentGroup`)))
  (bind _currentgroup_members_2 (break `/Game/Game/Blueprints/Enemy/S_EnemyGroup` (`local.CurrentGroup`)))
  (bind (_location _foundlocation) (`self.GetSpawnPoint`))
  (if _foundlocation
    (set `local.MainSpawnPoint` _location)
    (bind _id (`self.GetUnusedID`))
    (set `local.CurrentGroup` (make `/Game/Game/Blueprints/Enemy/S_EnemyGroup` _ _id))
    (for _ (range (+ (`KismetMathLibrary.RandomIntegerInRange` (`self.GroupMin`) (`self.GroupMax`)) 1))
      (bind _returnvalue (`|SpawnActorFromClass` "/Game/Game/Blueprints/Enemy/BP_Enemy.BP_Enemy_C" (`KismetMathLibrary.Conv_VectorToTransform` (`NavigationSystemV1.K2_GetRandomReachablePointInRadius` (`local.MainSpawnPoint`) 500.0 null null)) "AdjustIfPossibleButDontSpawnIfColliding" "MultiplyWithRoot" null null))
      (`/Engine/EditorBlueprintResources/StandardMacros.IsValid` _returnvalue
        (:`Is Valid`
          (set `/Game/Game/Blueprints/Enemy/BP_Enemy.Group` (`local.CurrentGroup`) _returnvalue)
          (`KismetArrayLibrary.Array_Add` _currentgroup_members_2 _returnvalue))))
    (bind _output_get (set `local.CurrentGroup` (make `/Game/Game/Blueprints/Enemy/S_EnemyGroup` _currentgroup_members _currentgroup_id (`|GetArrayItem` _currentgroup_members))))
    (for _array_element (`.Members_6_10290FF94D5B363314413F8ACE398828` (break `/Game/Game/Blueprints/Enemy/S_EnemyGroup` _output_get))
      (set `/Game/Game/Blueprints/Enemy/BP_Enemy.Group` _output_get _array_element))
    (`KismetArrayLibrary.Array_Add` (`self.Groups`) _output_get)))

(fn `UserConstructionScript`)