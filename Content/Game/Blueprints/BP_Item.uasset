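; BP_Item is a world pickup that shows an item's mesh and can be collected into a player's inventory.
; On BeginPlay and ID replication it looks up the ID in DT_Items, sets its Item struct and updates the static mesh.
; Tick bobs the mesh on a sine wave.
; Interacting adds the item ID to the player's InventoryComponent and destroys the actor if the add succeeds.
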(event `self.ReceiveBeginPlay`
  (bind (_returnvalue_x _returnvalue_y _returnvalue_z) (`KismetMathLibrary.BreakVector` (`self.K2_GetActorLocation`)))
  (`self.OnRep_ID`)
  (set `self.ZPosition` _returnvalue_z))

(event `self.ReceiveTick`
  (params (DeltaSeconds :type "Float (single-precision)"))
  (`SceneComponent.K2_SetRelativeLocation` (`self.StaticMesh`) (`KismetMathLibrary.MakeVector` 0.0 0.0 (+ (`self.ZPosition`) (* (`KismetMathLibrary.DegSin` (* (`self.GetGameTimeSinceCreation`) (`self.BobbingSpeed`))) (`self.BobbingDistance`)))) false false))

(event `Update`
  (bind (_item_name _item_description _item_thumbnail _item_staticmesh) (break `/Game/Game/S_Item` (`self.Item`)))
  (`StaticMeshComponent.SetStaticMesh` (`self.StaticMesh`) _item_staticmesh))

(event `OnInteract`
  (params (Player :type "/Game/Game/Blueprints/Characters/BP_BasePlayer Object Reference"))
  (`/Engine/EditorBlueprintResources/StandardMacros.IsValid` Player
    (:`Is Valid`
      (bind _newparam (`/Game/Game/InventoryComponent.Add` (`/Game/Game/Blueprints/Characters/BP_BasePlayer.InventoryComponent` Player) (`.ID_16_5564E16D4E89818FA1FFB6B410A76386` (break `/Game/Game/S_Item` (`self.Item`)))))
      (if _newparam
        (`self.K2_DestroyActor`)))))

(fn `Interact`
  (params (Player :type "/Game/Game/Blueprints/Characters/BP_BasePlayer Object Reference"))
  (returns (InteractID :type String))
  (`self.OnInteract` Player)
  (return (`self.InteractID`)))

(fn `OnRep_ID`
  (bind _returnvalue (`|GetDataTableRow` "/Game/Game/DT_Items.DT_Items" (`self.ID`))
    (:`then`
      (set `self.Item` (select `bool` (!= (`.ID_16_5564E16D4E89818FA1FFB6B410A76386` (break `/Game/Game/S_Item` (`self.Item`))) "None") :`false` _returnvalue))
      (`self.Update`))))

(fn `UserConstructionScript`)