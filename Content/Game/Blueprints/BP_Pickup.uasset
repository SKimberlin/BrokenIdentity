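; BP_Pickup is an item pickup actor that bobs in place and goes into a player's inventory on overlap.
; On BeginPlay or ID RepNotify it looks up ID in the ItemData table, lets a set DropItem override that row, and applies the item's static mesh.
; Tick drives the bobbing with a sine of game time.
; When a BP_BasePlayer overlaps, it destroys itself if the InventoryComponent accepts the item.
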(event `self.ReceiveBeginPlay`
  (bind (_returnvalue_x _returnvalue_y _returnvalue_z) (`KismetMathLibrary.BreakVector` (`self.K2_GetActorLocation`)))
  (`self.OnRep_ID`)
  (set `self.ZPosition` _returnvalue_z))

(event `self.ReceiveTick`
  (params (DeltaSeconds :type "Float (single-precision)"))
  (`SceneComponent.K2_SetRelativeLocation` (`self.StaticMesh`) (`KismetMathLibrary.MakeVector` 0.0 0.0 (+ (`self.ZPosition`) (* (`KismetMathLibrary.DegSin` (* (`self.GetGameTimeSinceCreation`) (`self.BobbingSpeed`))) (`self.BobbingDistance`)))) false false))

(event `Update`
  (bind (_item_name _item_description _item_thumbnail _item_staticmesh) (break `/Game/Game/S_Item` (`self.Item`)))
  (`StaticMeshComponent.SetStaticMesh` (`self.StaticMesh`) _item_staticmesh))

(event `self.ReceiveActorBeginOverlap`
  (params (OtherActor :type "Actor Object Reference"))
  (bind _asbp_base_player (cast `/Game/Game/Blueprints/Characters/BP_BasePlayer` OtherActor))
  (`/Engine/EditorBlueprintResources/StandardMacros.IsValid` _asbp_base_player
    (:`Is Valid`
      (bind _success (`/Game/Game/InventoryComponent.Add` (`/Game/Game/Blueprints/Characters/BP_BasePlayer.InventoryComponent` _asbp_base_player) (`self.ID`) (`self.Item`)))
      (if _success
        (`self.K2_DestroyActor`)))))

(fn `OnRep_ID`
  (bind _dropitem (`self.DropItem`))
  (bind _returnvalue (`|GetDataTableRow` "/Game/Game/ItemData.ItemData" (`self.ID`))
    (:`then`
      (set `self.Item` (select `bool` (!= (`.ID_16_5564E16D4E89818FA1FFB6B410A76386` (break `/Game/Game/S_Item` _dropitem)) "None") :`false` _returnvalue :`true` _dropitem))
      (`self.Update`))))

(fn `UserConstructionScript`)