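; Playable character Blueprint for Future, a melee fighter with light punch and elbow combos and heavy kick combos.
; Each attack input uses its combo counter to pick a montage, with completion or interruption resetting combo or attack state.
; The HitDetect override sphere-traces at the socket matching the current strike, damaging one BP_Enemy, adding ability and triggering hitstop on both characters.
; Debug prints, drawn traces and a max-health key remain.
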(event Input|EnhancedActionEvents|EnhancedInputActionIA_LightAttack
  (params (ActionValue :type Boolean) (ElapsedSeconds :type Float%20%28double-precision%29) (TriggeredSeconds :type Float%20%28double-precision%29) (InputAction :type Input%20Action%20Object%20Reference :default "/Game/ThirdPerson/Input/Actions/IA_LightAttack.IA_LightAttack"))
  (bind _charactermovement (Variables|Character|GetCharacterMovement))
  (bind _playerstatcomponent (Variables|Default|GetPlayerStatComponent))
  (if (not (Variables|Default|GetAttacking))
    (if (== (Variables|Default|GetLightAttackCount) (Variables|Default|GetLightAttackMax))
      (Variables|Default|SetLightAttackCount 0)
      (else
        (CallFunction|AttackDirectionHelper)
        (Animation|Montage|PlayMontage (Variables|Character|GetMesh) (Utilities|Select :Index (Variables|Default|GetLightAttackCount) :Option%200 "/Game/Game/Animations/FullMelee/Attacks/Punches/Cross_Punch_Montage.Cross_Punch_Montage" :Option%201 "/Game/Game/Animations/FullMelee/Attacks/Punches/Elbow_Punching_Montage.Elbow_Punching_Montage" :Option%202 "/Game/Game/Animations/FullMelee/Attacks/Punches/Hook__3__Montage.Hook__3__Montage" :Option%203 "/Game/Game/Animations/FullMelee/Attacks/Punches/Hook__2__Montage.Hook__2__Montage" :Option%204 "/Game/Game/Animations/FullMelee/Attacks/Punches/Hook_Montage.Hook_Montage" :Option%205 "/Game/Game/Animations/FullMelee/Attacks/Punches/Hook__1__Montage.Hook__1__Montage" :Option%206 "/Game/Game/Animations/FullMelee/Attacks/Punches/Elbow_Punching_Montage.Elbow_Punching_Montage" :Option%207 0 :Option%208 0)
          (:then
            (Variables|Default|SetAttacking true)
            (bind _result (Math|Integer|IncrementInt (Variables|Default|GetLightAttackCount))
              (:%20%20
                (Variables|Default|SetCanMove true)
                (Variables|/Script/Engine.CharacterMovementComponent|SetMaxWalkSpeed _charactermovement (Variables|/Game/Game/CharacterStatComponent.CharacterStatComponent_C|GetRunSpeed _playerstatcomponent))
                (switch int _result
                  (:1
                    (Development|PrintString "1"))
                  (:2
                    (Development|PrintString "2"))
                  (:3
                    (Development|PrintString "3"))
                  (:4
                    (Development|PrintString "4"))
                  (:5
                    (Development|PrintString "5"))))))
          (:OnCompleted
            (Variables|Default|SetLightAttackCount 0)
            (Variables|Default|SetCanMove true :!label _label)
            (Variables|/Script/Engine.CharacterMovementComponent|SetMaxWalkSpeed _charactermovement (Variables|/Game/Game/CharacterStatComponent.CharacterStatComponent_C|GetWalkSpeed _playerstatcomponent)))
          (:OnInterrupted
            (Variables|Default|SetAttacking false)
            (goto _label)))))))

(event Input|EnhancedActionEvents|EnhancedInputActionIA_HeavyAttack
  (params (ActionValue :type Boolean) (ElapsedSeconds :type Float%20%28double-precision%29) (TriggeredSeconds :type Float%20%28double-precision%29) (InputAction :type Input%20Action%20Object%20Reference :default "/Game/ThirdPerson/Input/Actions/IA_HeavyAttack.IA_HeavyAttack"))
  (if (not (Variables|Default|GetAttacking))
    (if (== (Variables|Default|GetHeavyAttackCount) (Variables|Default|GetHeavyAttackMax))
      (Variables|Default|SetHeavyAttackCount 0)
      (else
        (CallFunction|AttackDirectionHelper)
        (Animation|Montage|PlayMontage (Variables|Character|GetMesh) (Utilities|Select :Index (Variables|Default|GetHeavyAttackCount) :Option%200 "/Game/Game/Animations/FullMelee/Attacks/Kicks/Mma_Kick__1__Montage.Mma_Kick__1__Montage" :Option%201 "/Game/Game/Animations/FullMelee/Attacks/Kicks/Mma_Kick__2__Montage.Mma_Kick__2__Montage" :Option%202 "/Game/Game/Animations/FullMelee/Attacks/Kicks/Mma_Kick_Montage.Mma_Kick_Montage" :Option%203 "/Game/Game/Animations/FullMelee/Attacks/Kicks/Roundhouse_Kick_Montage.Roundhouse_Kick_Montage" :Option%204 "/Game/Game/Animations/FullMelee/Attacks/Kicks/Mma_Kick__3__Montage.Mma_Kick__3__Montage" :Option%205 "/Game/Game/Animations/FullMelee/Attacks/Kicks/Roundhouse_Kick_Montage.Roundhouse_Kick_Montage" :Option%206 0 :Option%207 0 :Option%208 0)
          (:then
            (Variables|Default|SetAttacking true)
            (bind _result (Math|Integer|IncrementInt (Variables|Default|GetHeavyAttackCount))
              (:%20%20
                (Variables|Default|SetInHeavy true)
                (switch int _result
                  (:1
                    (Development|PrintString "1"))
                  (:2
                    (Development|PrintString "2"))
                  (:3
                    (Development|PrintString "3"))
                  (:4
                    (Development|PrintString "4"))
                  (:5
                    (Development|PrintString "5"))))))
          (:OnCompleted
            (Variables|Default|SetHeavyAttackCount 0))
          (:OnInterrupted
            (Variables|Default|SetAttacking false)
            (Variables|Default|SetInHeavy false)))))))

(event EventBeginPlay
  (|CallParentFunction) ; This node is disabled and will not be called.\nDrag off pins to build functionality.
)

(event Collision|EventActorBeginOverlap
  (params (OtherActor :type Actor%20Object%20Reference))
  (|CallParentFunction OtherActor) ; This node is disabled and will not be called.\nDrag off pins to build functionality.
)

(event EventTick
  (params (DeltaSeconds :type Float%20%28single-precision%29))
  (|CallParentFunction DeltaSeconds) ; This node is disabled and will not be called.\nDrag off pins to build functionality.
)

(event Input|KeyboardEvents|DebugKeyN
  (params (Key :type Key%20Structure) (ActionValue :type Input%20Action%20Value%20Structure))
  (:Pressed
    (CallFunction|UpdateMaxHealth 5e+01)))

(fn ConstructionScript
  (|CallParentFunction))

(fn HitDetect
  (|CallParentFunction)
  (if (not (Variables|Default|GetHitTarget))
    (if (Variables|Default|GetInHeavy)
      (LocalVariables|SetSphereLocation (Transformation|GetSocketLocation (Variables|Character|GetMesh) (Utilities|Select :Index (Variables|Default|GetHeavyAttackCount) :Option%200 "foot_r" :Option%201 "foot_r" :Option%202 "foot_l" :Option%203 "foot_r" :Option%204 "foot_r")))
      (else
        (LocalVariables|SetSphereLocation (Transformation|GetSocketLocation (Variables|Character|GetMesh) (Utilities|Select :Index (Variables|Default|GetLightAttackCount) :Option%200 "hand_r" :Option%201 "lowerarm_correctiveRoot_r" :Option%202 "hand_l" :Option%203 "hand_l" :Option%204 "hand_l" :Option%205 "hand_l" :Option%206 "lowerarm_correctiveRoot_r")))))
    (bind _outhit (Collision|SphereTraceForObjects (LocalVariables|GetSphereLocation) (LocalVariables|GetSphereLocation) 4e+01 (Utilities|Array|MakeArray "ObjectTypeQuery3") false 0 "ForDuration"))
    (bind _asbp_enemy (Utilities|Casting|CastToBP_Enemy (.HitActor (Collision|BreakHitResult _outhit))))
    (Game|Damage|ApplyDamage _asbp_enemy 1e+01 0 self "/Script/Engine.DamageType")
    (Variables|Default|SetHitTarget true)
    (CallFunction|AddAbility 1e+01)
    (Default|StartHitstop (Variables|Default|GetHitstopComponent) 0.1)
    (Default|StartHitstop (Variables|/Game/Game/Blueprints/Enemy/BP_Enemy.BP_Enemy_C|GetHitstopComponent _asbp_enemy) 0.1)))