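; Test character variant that prototypes a light and heavy attack combo driven by input actions.
; Light attacks count up to a cap, blocked during heavies or a running animation timer, alternating right and left hit montages before later hits only print debug text.
; Heavy attacks branch by light count into three currently identical tiers that print and set InHeavy.
; Attacks set a chain timer, but nothing here counts down timers or resets combos.
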(event `EnhancedInput|/Game/ThirdPerson/Input/Actions/IA_LightAttack`
  (params (ActionValue :type Boolean) (ElapsedSeconds :type "Float (double-precision)") (TriggeredSeconds :type "Float (double-precision)") (InputAction :type "InputAction Object Reference" :default "/Game/ThirdPerson/Input/Actions/IA_LightAttack.IA_LightAttack"))
  (bind _lightattackcount (`self.LightAttackCount`))
  (:`Triggered`
    (if (not (or (== _lightattackcount (`self.LightAttackMax`)) (`self.InHeavy`) (>= (`self.AnimationTimer`) 0.0)))
      (bind _result (`/Engine/EditorBlueprintResources/StandardMacros.IncrementInt` _lightattackcount)
        (:`  `
          (switch `int` _result
            (:`1`
              (bind _returnvalue (`self.PlayAnimMontage` "/Game/Game/Animations/HitRight.HitRight" :!label _label))
              (set `self.AnimationTimer` (- _returnvalue 2.0))
              (set `self.ChainTimer` (+ _returnvalue 0.5)))
            (:`2`
              (bind _returnvalue_2 (`self.PlayAnimMontage` "/Game/Game/Animations/HitLeft.HitLeft" :!label _label_2))
              (set `self.AnimationTimer` (- _returnvalue_2 1.0))
              (set `self.ChainTimer` (+ _returnvalue_2 0.5)))
            (:`3`
              (goto _label))
            (:`4`
              (goto _label_2))
            (:`5`
              (goto _label))
            (:`6`
              (`KismetSystemLibrary.PrintString` (`KismetStringLibrary.BuildString_Int` "" "Light x" _result) :!label _label_3)
              (set `self.ChainTimer` 1.0 :!label _label_4))
            (:`7`
              (goto _label_3))
            (:`8`
              (goto _label_3))))))))

(event `EnhancedInput|/Game/ThirdPerson/Input/Actions/IA_HeavyAttack`
  (params (ActionValue :type Boolean) (ElapsedSeconds :type "Float (double-precision)") (TriggeredSeconds :type "Float (double-precision)") (InputAction :type "InputAction Object Reference" :default "/Game/ThirdPerson/Input/Actions/IA_HeavyAttack.IA_HeavyAttack"))
  (bind _heavyattackcount (`self.HeavyAttackCount`))
  (bind _returnvalue (== _heavyattackcount (`self.HeavyAttackMax`)))
  (:`Triggered`
    (switch `int` (`self.LightAttackCount`)
      (:`0`
        (if (not _returnvalue) :!label _label_5
          (bind _result (`/Engine/EditorBlueprintResources/StandardMacros.IncrementInt` _heavyattackcount)
            (:`  `
              (switch `int` _result
                (:`0`
                  _)
                (:`1`
                  _)
                (:`2`
                  _))
              (`KismetSystemLibrary.PrintString` (`KismetStringLibrary.BuildString_Int` "" "Heavy x" _heavyattackcount) :!label _label_6)
              (set `self.InHeavy` true)
              (goto _label_4)))))
      (:`1`
        (goto _label_5))
      (:`2`
        (goto _label_5))
      (:`3`
        (if (not _returnvalue) :!label _label_7
          (bind _result_2 (`/Engine/EditorBlueprintResources/StandardMacros.IncrementInt` _heavyattackcount)
            (:`  `
              (switch `int` _result_2
                (:`0`
                  (goto _label_6))
                (:`1`
                  (goto _label_6))
                (:`2`
                  (goto _label_6)))))))
      (:`4`
        (goto _label_7))
      (:`5`
        (goto _label_7))
      (:`6`
        (if (not _returnvalue) :!label _label_8
          (bind _result_3 (`/Engine/EditorBlueprintResources/StandardMacros.IncrementInt` _heavyattackcount)
            (:`  `
              (switch `int` _result_3
                (:`0`
                  (goto _label_6))
                (:`1`
                  (goto _label_6))
                (:`2`
                  (goto _label_6)))))))
      (:`7`
        (goto _label_8))
      (:`8`
        (goto _label_8)))))

(fn `UserConstructionScript`
  (`parent.UserConstructionScript`))