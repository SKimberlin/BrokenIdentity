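; Crowd NPC that assembles a randomized modular human look in its Construction Script, with no active event logic.
; Face, shirt, pants and shoes follow the body mesh through leader pose.
; A random pick of two female and two male body types sets face and body meshes, then clothing from gender-specific lists.
; GroomBind draws hair from per-body-type lists, with separate Random calls for groom and binding, so the two can mismatch.
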(fn `GroomBind`
  (locals (`f_001 hair` :type "Array of /Game/Game/Blueprints/NPC/S_Hair Structure") (`f_002 hair` :type "Array of /Game/Game/Blueprints/NPC/S_Hair Structure") (`m_001 hair` :type "Array of /Game/Game/Blueprints/NPC/S_Hair Structure") (`m_002 hair` :type "Array of /Game/Game/Blueprints/NPC/S_Hair Structure"))
  (bind _hair (`self.Hair`))
  (bind _hair_2 (`self.Hair`))
  (bind _hair_3 (`self.Hair`))
  (bind _hair_4 (`self.Hair`))
  (bind _outitem (`KismetArrayLibrary.Array_Random` (`local.m_002 hair`)))
  (bind _outitem_2 (`KismetArrayLibrary.Array_Random` (`local.f_001 hair`)))
  (bind _outitem_3 (`KismetArrayLibrary.Array_Random` (`local.f_002 hair`)))
  (bind _outitem_4 (`KismetArrayLibrary.Array_Random` (`local.m_001 hair`)))
  (switch `/Game/Game/Blueprints/NPC/E_BodyType` (`self.BodyType`)
    (:`NewEnumerator0`
      (`GroomComponent.SetGroomAsset` _hair_2 (break `/Game/Game/Blueprints/NPC/S_Hair` _outitem_2))
      (`GroomComponent.SetBindingAsset` _hair_2 (`.BindingAsset_5_AFBB5A144701D3684477AFA666C44E6C` (break `/Game/Game/Blueprints/NPC/S_Hair` _outitem_2))))
    (:`NewEnumerator1`
      (`GroomComponent.SetGroomAsset` _hair_3 (break `/Game/Game/Blueprints/NPC/S_Hair` _outitem_3))
      (`GroomComponent.SetBindingAsset` _hair_3 (`.BindingAsset_5_AFBB5A144701D3684477AFA666C44E6C` (break `/Game/Game/Blueprints/NPC/S_Hair` _outitem_3))))
    (:`NewEnumerator6`
      (`GroomComponent.SetGroomAsset` _hair_4 (break `/Game/Game/Blueprints/NPC/S_Hair` _outitem_4))
      (`GroomComponent.SetBindingAsset` _hair_4 (`.BindingAsset_5_AFBB5A144701D3684477AFA666C44E6C` (break `/Game/Game/Blueprints/NPC/S_Hair` _outitem_4))))
    (:`NewEnumerator7`
      (`GroomComponent.SetGroomAsset` _hair (break `/Game/Game/Blueprints/NPC/S_Hair` _outitem))
      (`GroomComponent.SetBindingAsset` _hair (`.BindingAsset_5_AFBB5A144701D3684477AFA666C44E6C` (break `/Game/Game/Blueprints/NPC/S_Hair` _outitem))))))

(fn `UserConstructionScript`
  (locals (MaleClothes :type "/Game/Game/Blueprints/NPC/S_Clothes Structure" :default (struct :`Shirts` "(\"/Script/Engine.SkeletalMesh'/Game/CitySampleCrowd/Character/Male/NormalWeight/Meshes/m_tal_nrw_buttonDown.m_tal_nrw_buttonDown'\",\"/Script/Engine.SkeletalMesh'/Game/CitySampleCrowd/Character/Male/NormalWeight/Meshes/m_tal_nrw_buttonDown_blazer.m_tal_nrw_buttonDown_blazer'\",\"/Script/Engine.SkeletalMesh'/Game/CitySampleCrowd/Character/Male/NormalWeight/Meshes/m_tal_nrw_buttonDown_blazer.m_tal_nrw_buttonDown_blazer'\",\"/Script/Engine.SkeletalMesh'/Game/CitySampleCrowd/Character/Male/NormalWeight/Meshes/m_tal_nrw_buttonDown_tie.m_tal_nrw_buttonDown_tie'\",\"/Script/Engine.SkeletalMesh'/Game/CitySampleCrowd/Character/Male/NormalWeight/Meshes/m_tal_nrw_crewneck.m_tal_nrw_crewneck'\",\"/Script/Engine.SkeletalMesh'/Game/CitySampleCrowd/Character/Male/NormalWeight/Meshes/m_tal_nrw_buttonOpen.m_tal_nrw_buttonOpen'\")" :`Pants` "(\"/Script/Engine.SkeletalMesh'/Game/CitySampleCrowd/Character/Male/NormalWeight/Meshes/m_tal_nrw_jeans.m_tal_nrw_jeans'\",\"/Script/Engine.SkeletalMesh'/Game/CitySampleCrowd/Character/Male/NormalWeight/Meshes/m_tal_nrw_slacks.m_tal_nrw_slacks'\",\"/Script/Engine.SkeletalMesh'/Game/CitySampleCrowd/Character/Male/NormalWeight/Meshes/m_tal_nrw_jeansLong.m_tal_nrw_jeansLong'\")" :`Shoes` "(\"/Script/Engine.SkeletalMesh'/Game/CitySampleCrowd/Character/Male/NormalWeight/Meshes/m_tal_nrw_loafers.m_tal_nrw_loafers'\",\"/Script/Engine.SkeletalMesh'/Game/CitySampleCrowd/Character/Male/NormalWeight/Meshes/m_tal_nrw_oxfords.m_tal_nrw_oxfords'\")")) (FemaleClothes :type "/Game/Game/Blueprints/NPC/S_Clothes Structure" :default (struct :`Shirts` "(\"/Script/Engine.SkeletalMesh'/Game/CitySampleCrowd/Character/Female/NormalWeight/Meshes/f_tal_nrw_buttonDown.f_tal_nrw_buttonDown'\",\"/Script/Engine.SkeletalMesh'/Game/CitySampleCrowd/Character/Female/NormalWeight/Meshes/f_tal_nrw_buttonOpen_blazer.f_tal_nrw_buttonOpen_blazer'\",\"/Script/Engine.SkeletalMesh'/Game/CitySampleCrowd/Character/Female/NormalWeight/Meshes/f_tal_nrw_scoopneck.f_tal_nrw_scoopneck'\",\"/Script/Engine.SkeletalMesh'/Game/CitySampleCrowd/Character/Female/NormalWeight/Meshes/f_tal_nrw_turtleneck.f_tal_nrw_turtleneck'\")" :`Pants` "(\"/Script/Engine.SkeletalMesh'/Game/CitySampleCrowd/Character/Female/NormalWeight/Meshes/f_tal_nrw_jeans.f_tal_nrw_jeans'\",\"/Script/Engine.SkeletalMesh'/Game/CitySampleCrowd/Character/Female/NormalWeight/Meshes/f_tal_nrw_slacks.f_tal_nrw_slacks'\",\"/Script/Engine.SkeletalMesh'/Game/CitySampleCrowd/Character/Female/NormalWeight/Meshes/f_tal_nrw_skirt.f_tal_nrw_skirt'\")" :`Shoes` "(\"/Script/Engine.SkeletalMesh'/Game/CitySampleCrowd/Character/Female/NormalWeight/Meshes/f_tal_nrw_dressFlats.f_tal_nrw_dressFlats'\",\"/Script/Engine.SkeletalMesh'/Game/CitySampleCrowd/Character/Female/NormalWeight/Meshes/f_tal_nrw_loafers.f_tal_nrw_loafers'\",\"/Script/Engine.SkeletalMesh'/Game/CitySampleCrowd/Character/Female/NormalWeight/Meshes/f_tal_nrw_oxfords.f_tal_nrw_oxfords'\")")))
  (bind (_maleclothes_shirts _maleclothes_pants _maleclothes_shoes) (break `/Game/Game/Blueprints/NPC/S_Clothes` (`local.MaleClothes`)))
  (bind (_femaleclothes_shirts _femaleclothes_pants _femaleclothes_shoes) (break `/Game/Game/Blueprints/NPC/S_Clothes` (`local.FemaleClothes`)))
  (`|ExecutionSequence`
    (:`then_0`
      (`SkinnedMeshComponent.SetLeaderPoseComponent` (`self.Pants`) (`self.Mesh`) false false)
      (`SkinnedMeshComponent.SetLeaderPoseComponent` (`self.Shoes`) (`self.Mesh`) false false)
      (`SkinnedMeshComponent.SetLeaderPoseComponent` (`self.Face`) (`self.Mesh`) false false)
      (`SkinnedMeshComponent.SetLeaderPoseComponent` (`self.Shirt`) (`self.Mesh`) false false))
    (:`then_1`
      (bind _output_get (set `self.BodyType` (select `int` (`KismetMathLibrary.RandomInteger` 4) :`0` "NewEnumerator0" :`1` "NewEnumerator1" :`2` "NewEnumerator6" :`3` "NewEnumerator7" :!type "/Game/Game/Blueprints/NPC/E_BodyType Enum")))
      (`SkeletalMeshComponent.SetSkeletalMeshAsset` (`self.Face`) (select `/Game/Game/Blueprints/NPC/E_BodyType` _output_get :`NewEnumerator0` "/Game/CitySampleCrowd/Character/Female/f_001/Face/f_001_nrw_FaceMesh.f_001_nrw_FaceMesh" :`NewEnumerator1` "/Game/CitySampleCrowd/Character/Female/f_002/Face/f_002_nrw_FaceMesh.f_002_nrw_FaceMesh" :`NewEnumerator6` "/Game/CitySampleCrowd/Character/Male/m_001/Face/m_001_nrw_FaceMesh.m_001_nrw_FaceMesh" :`NewEnumerator7` "/Game/CitySampleCrowd/Character/Male/m_002/Face/m_002_nrw_FaceMesh.m_002_nrw_FaceMesh" :!type "SkeletalMesh Object Reference"))
      (`SkeletalMeshComponent.SetSkeletalMeshAsset` (`self.Mesh`) (select `/Game/Game/Blueprints/NPC/E_BodyType` _output_get :`NewEnumerator0` "/Game/CitySampleCrowd/Character/Female/NormalWeight/Meshes/f_tal_nrw_body.f_tal_nrw_body" :`NewEnumerator1` "/Game/CitySampleCrowd/Character/Female/NormalWeight/Meshes/f_tal_nrw_body.f_tal_nrw_body" :`NewEnumerator6` "/Game/CitySampleCrowd/Character/Male/NormalWeight/Meshes/m_tal_nrw_body.m_tal_nrw_body" :`NewEnumerator7` "/Game/CitySampleCrowd/Character/Male/NormalWeight/Meshes/m_tal_nrw_body.m_tal_nrw_body" :!type "SkeletalMesh Object Reference"))
      (`self.GroomBind`)
      (switch `/Game/Game/Blueprints/NPC/E_BodyType` _output_get
        (:`NewEnumerator0`
          (`SkeletalMeshComponent.SetSkeletalMeshAsset` (`self.Shirt`) (`KismetArrayLibrary.Array_Random` _femaleclothes_shirts) :!label _label)
          (`SkeletalMeshComponent.SetSkeletalMeshAsset` (`self.Pants`) (`KismetArrayLibrary.Array_Random` _femaleclothes_pants))
          (`SkeletalMeshComponent.SetSkeletalMeshAsset` (`self.Shoes`) (`KismetArrayLibrary.Array_Random` _femaleclothes_shoes)))
        (:`NewEnumerator1`
          (goto _label))
        (:`NewEnumerator6`
          (`SkeletalMeshComponent.SetSkeletalMeshAsset` (`self.Shirt`) (`KismetArrayLibrary.Array_Random` _maleclothes_shirts) :!label _label_2)
          (`SkeletalMeshComponent.SetSkeletalMeshAsset` (`self.Pants`) (`KismetArrayLibrary.Array_Random` _maleclothes_pants))
          (`SkeletalMeshComponent.SetSkeletalMeshAsset` (`self.Shoes`) (`KismetArrayLibrary.Array_Random` _maleclothes_shoes)))
        (:`NewEnumerator7`
          (goto _label_2))))))