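; ShopComponent is an NPC shop component that lets the player buy items through a shop menu.
; On BeginPlay it resolves its item IDs against DT_Items; ToggleShop opens WBP_ShopMenu with that stock and pauses the game, or closes it and unpauses.
; Cart functions track open inventory slots and running cost against the player's money.
; PurchaseItems adds the cart to the player's inventory, deducts the total and empties the cart.
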(event `self.ReceiveBeginPlay`
  (for _array_element (`self.SellingItemIDs`)
    (bind _returnvalue (`|GetDataTableRow` "/Game/Game/DT_Items.DT_Items" _array_element)
      (:`then`
        (`KismetArrayLibrary.Array_Add` (`self.SellingItems`) _returnvalue)))))

(event `ToggleShop`
  (bind _output_get (set `self.Player` (cast `/Game/Game/Blueprints/Characters/BP_BasePlayer` (`GameplayStatics.GetPlayerPawn` 0) :!pure true)))
  (`/Engine/EditorBlueprintResources/StandardMacros.IsValid` (`self.MenuWidget`)
    (:`Is Valid`
      (`Widget.RemoveFromParent` (`self.MenuWidget`))
      (set `self.MenuWidget` null)
      (`KismetSystemLibrary.CollectGarbage`)
      (`GameplayStatics.SetGamePaused` false))
    (:`Is Not Valid`
      (bind _inventorycomponent (`/Game/Game/Blueprints/Characters/BP_BasePlayer.InventoryComponent` _output_get))
      (bind _available (`/Game/Game/InventoryComponent.Slots Available` _inventorycomponent))
      (set `self.OpenSlots` _available)
      (bind _returnvalue (`|CreateWidget` "/Game/Game/Blueprints/Widgets/WBP_ShopMenu.WBP_ShopMenu_C" null self _inventorycomponent (`self.SellingItems`)))
      (bind _output_get_2 (set `self.MenuWidget` _returnvalue))
      (`UserWidget.AddToViewport` _output_get_2 0)
      (`GameplayStatics.SetGamePaused` true))))

(fn `AddToCart`
  (params (Item :type "/Game/Game/S_Item Structure"))
  (returns (Added :type Boolean))
  (bind _openslots (`self.OpenSlots`))
  (bind _returnvalue (+ (`self.TotalCartCost`) (`.Value_28_D4D3FFDF4A269EB9D5F1548AE741D803` (break `/Game/Game/S_Item` Item))))
  (if (> _openslots 0)
    (if (<= _returnvalue (`/Game/Game/InventoryComponent.Money` (`/Game/Game/Blueprints/Characters/BP_BasePlayer.InventoryComponent` (`self.Player`))))
      (`KismetArrayLibrary.Array_Add` (`self.Cart`) Item)
      (`/Engine/EditorBlueprintResources/StandardMacros.DecrementInt` _openslots
        (:`  `
          (set `self.TotalCartCost` _returnvalue)
          (return true)))
      (else
        _)))
  (return false))

(fn `CanAfford`
  (returns (Afford :type Boolean))
  (return (>= (`/Game/Game/InventoryComponent.Money` (`/Game/Game/Blueprints/Characters/BP_BasePlayer.InventoryComponent` (`self.Player`))) (`self.TotalCartCost`))))

(fn `PurchaseItems`
  (bind _cart (`self.Cart`))
  (bind _player (`self.Player`))
  (for _array_element _cart
    (`/Game/Game/InventoryComponent.Add` (`/Game/Game/Blueprints/Characters/BP_BasePlayer.InventoryComponent` _player) (`.ID_16_5564E16D4E89818FA1FFB6B410A76386` (break `/Game/Game/S_Item` _array_element))))
  (`/Game/Game/Blueprints/Characters/BP_BasePlayer.RemoveMoney` _player (`self.TotalCartCost`))
  (`KismetArrayLibrary.Array_Clear` _cart))

(fn `RemoveFromCart`
  (params (Index :type Integer))
  (bind _cart (`self.Cart`))
  (bind (_output_name _output_description _output_thumbnail _output_staticmesh _output_id _output_type _output_consumeeffect _output_value) (break `/Game/Game/S_Item` (`|GetArrayItem` _cart Index)))
  (set `self.TotalCartCost` (- (`self.TotalCartCost`) _output_value))
  (`KismetArrayLibrary.Array_Remove` _cart Index)
  (`/Engine/EditorBlueprintResources/StandardMacros.IncrementInt` (`self.OpenSlots`)))