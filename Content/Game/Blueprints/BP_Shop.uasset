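; Interactable shop actor that sells items listed by ID, resolved from DT_Items on BeginPlay.
; Interact toggles WBP_ShopMenu, pausing the game and switching input mode and cursor.
; Cart functions track total cost and open inventory slots; CanAfford compares that total to player money.
; PurchaseItems adds cart items to the inventory and empties the cart, but passes zero to RemoveMoney and never resets the total.
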(event `self.ReceiveBeginPlay`
  (bind _aswbp_interact (cast `/Game/Game/Blueprints/Widgets/WBP_Interact` (`WidgetComponent.GetWidget` (`self.Widget`))))
  (set `/Game/Game/Blueprints/Widgets/WBP_Interact.Text` "to Shop" _aswbp_interact)
  (for _array_element (`self.SellingItemIDs`)
    (bind _returnvalue (`|GetDataTableRow` "/Game/Game/DT_Items.DT_Items" _array_element)
      (:`then`
        (`KismetArrayLibrary.Array_Add` (`self.SellingItems`) _returnvalue)))))

(event `/Game/Game/Blueprints/BPI_Interactable.Interact`
  (params (Player :type "/Game/Game/Blueprints/Characters/BP_BasePlayer Object Reference"))
  (bind _returnvalue (`Pawn.GetController` Player))
  (bind _inventorycomponent (`/Game/Game/Blueprints/Characters/BP_BasePlayer.InventoryComponent` Player))
  (set `self.Player` Player)
  (`/Engine/EditorBlueprintResources/StandardMacros.IsValid` (`self.MenuWidget`)
    (:`Is Valid`
      (`Widget.RemoveFromParent` (`self.MenuWidget`))
      (set `self.MenuWidget` null)
      (`KismetSystemLibrary.CollectGarbage`)
      (bind _asplayer_controller (cast `PlayerController` _returnvalue))
      (`WidgetBlueprintLibrary.SetInputMode_GameOnly` _asplayer_controller)
      (`GameplayStatics.SetGamePaused` false)
      (set `PlayerController.bShowMouseCursor` false _asplayer_controller))
    (:`Is Not Valid`
      (bind _available (`/Game/Game/InventoryComponent.Slots Available` _inventorycomponent))
      (set `self.OpenSlots` _available)
      (bind _returnvalue_2 (`|CreateWidget` "/Game/Game/Blueprints/Widgets/WBP_ShopMenu.WBP_ShopMenu_C" null self _inventorycomponent (`self.SellingItems`)))
      (bind _output_get (set `self.MenuWidget` _returnvalue_2))
      (`UserWidget.AddToViewport` _output_get 0)
      (bind _asplayer_controller_2 (cast `PlayerController` _returnvalue))
      (`WidgetBlueprintLibrary.SetInputMode_GameAndUIEx` _asplayer_controller_2 null "DoNotLock" false)
      (`GameplayStatics.SetGamePaused` true)
      (set `PlayerController.bShowMouseCursor` true _asplayer_controller_2))))

(fn `AddToCart`
  (params (Item :type "/Game/Game/S_Item Structure"))
  (returns (Added :type Boolean))
  (bind _openslots (`self.OpenSlots`))
  (if (> _openslots 0)
    (`KismetArrayLibrary.Array_Add` (`self.Cart`) Item)
    (`/Engine/EditorBlueprintResources/StandardMacros.DecrementInt` _openslots
      (:`  `
        (set `self.TotalCartCost` (+ (`self.TotalCartCost`) (`.Value_28_D4D3FFDF4A269EB9D5F1548AE741D803` (break `/Game/Game/S_Item` Item))))
        (return true)))
    (else
      (return false))))

(fn `CanAfford`
  (returns (Afford :type Boolean))
  (return (>= (`/Game/Game/PlayerStatComponent.Money` (`/Game/Game/Blueprints/Characters/BP_BasePlayer.PlayerStatComponent` (`self.Player`))) (`self.TotalCartCost`))))

(fn `PurchaseItems`
  (bind _cart (`self.Cart`))
  (bind _player (`self.Player`))
  (for _array_element _cart
    (`/Game/Game/InventoryComponent.Add` (`/Game/Game/Blueprints/Characters/BP_BasePlayer.InventoryComponent` _player) (`.ID_16_5564E16D4E89818FA1FFB6B410A76386` (break `/Game/Game/S_Item` _array_element))))
  (`/Game/Game/Blueprints/Characters/BP_BasePlayer.RemoveMoney` _player 0)
  (`KismetArrayLibrary.Array_Clear` _cart))

(fn `RemoveFromCart`
  (params (Index :type Integer))
  (bind _cart (`self.Cart`))
  (bind (_output_name _output_description _output_thumbnail _output_staticmesh _output_id _output_type _output_consumeeffect _output_value) (break `/Game/Game/S_Item` (`|GetArrayItem` _cart Index)))
  (set `self.TotalCartCost` (- (`self.TotalCartCost`) _output_value))
  (`KismetArrayLibrary.Array_Remove` _cart Index)
  (`/Engine/EditorBlueprintResources/StandardMacros.IncrementInt` (`self.OpenSlots`)))

(fn `UserConstructionScript`)