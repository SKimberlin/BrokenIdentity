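; Base quest actor that tracks one quest's objective progress through its stages.
; On BeginPlay it loads its QuestData row by ID, zeroes the current stage's objective counts and binds to the player's interact-ID event.
; Matching interactions add to progress until the required quantity is reached.
; When all objectives are met it advances the stage, marking the quest complete if the new stage's first objective ID is empty.
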(event `self.ReceiveBeginPlay`
  (`self.GetQuestDetails`)
  (add `/Game/Game/Blueprints/Characters/BP_BasePlayer.OnInteractIDCalled` (cast `/Game/Game/Blueprints/Characters/BP_BasePlayer` (`GameplayStatics.GetPlayerCharacter` 0) :!pure true) (delegate `OnInteractIDHeard`))
  (`self.AllObjectivesComplete`))

(event `OnInteractIDHeard`
  (params (InteractID :type String) (Value :type Integer))
  (bind _objectiveprogress (`self.ObjectiveProgress`))
  (bind (_value _returnvalue) (`BlueprintMapLibrary.Map_Find` _objectiveprogress InteractID))
  (if _returnvalue
    (if (< _value (`.Quantity_12_E82C91294D60ACD3A26E7CB866C7DD17` (break `/Game/Game/Blueprints/Quests/S_QuestObjective` (`self.GetObjectiveDataByID` InteractID))))
      (`BlueprintMapLibrary.Map_Add` _objectiveprogress InteractID (+ _value Value))
      (`self.AllObjectivesComplete`))))

(fn `AllObjectivesComplete`
  (for _array_element (`.Objectives_19_477E79AE4F539C86C339C682D01F5F05` (break `/Game/Game/Blueprints/Quests/S_QuestStage` (`self.StageDetails`)))
    (bind (_name _description _type _id) (break `/Game/Game/Blueprints/Quests/S_QuestObjective` _array_element))
    (if (not (>= (`BlueprintMapLibrary.Map_Find` (`self.ObjectiveProgress`) _id) (`.Quantity_12_E82C91294D60ACD3A26E7CB866C7DD17` (break `/Game/Game/Blueprints/Quests/S_QuestObjective` (`self.GetObjectiveDataByID` _id)))))
      (return)))
  (bind _result (`/Engine/EditorBlueprintResources/StandardMacros.IncrementInt` (`self.Stage`))
    (:`  `
      (bind _output (`|GetArrayItem` (`.Stages_15_2D92E51C4F3B62A5376D7089B683056B` (break `/Game/Game/Blueprints/Quests/S_QuestDetails` (`self.QuestDetails`))) _result))
      (set `self.StageDetails` _output)
      (set `self.Complete` (`KismetStringLibrary.EqualEqual_StrStr` (`.ID_9_57A6F44044E56A75E66920BB7B4CBE21` (break `/Game/Game/Blueprints/Quests/S_QuestObjective` (`|GetArrayItem` (`.Objectives_19_477E79AE4F539C86C339C682D01F5F05` (break `/Game/Game/Blueprints/Quests/S_QuestStage` _output))))))))))

(fn `GetObjectiveDataByID`
  (params (ID :type String))
  (returns (`Array Element` :type "/Game/Game/Blueprints/Quests/S_QuestObjective Structure"))
  (for _array_element (`.Objectives_19_477E79AE4F539C86C339C682D01F5F05` (break `/Game/Game/Blueprints/Quests/S_QuestStage` (`self.StageDetails`)))
    (if (`KismetStringLibrary.EqualEqual_StrStr` (`.ID_9_57A6F44044E56A75E66920BB7B4CBE21` (break `/Game/Game/Blueprints/Quests/S_QuestObjective` _array_element)) ID)
      (return _array_element))))

(fn `GetQuestDetails`
  (bind _returnvalue (`|GetDataTableRow` "/Game/Game/Blueprints/Quests/QuestData.QuestData" (`self.ID`))
    (:`then`
      (bind _output_get (set `self.QuestDetails` _returnvalue))
      (bind _output_get_2 (set `self.StageDetails` (`|GetArrayItem` (`.Stages_15_2D92E51C4F3B62A5376D7089B683056B` (break `/Game/Game/Blueprints/Quests/S_QuestDetails` _output_get)) (`self.Stage`))))
      (`BlueprintMapLibrary.Map_Clear` (`self.ObjectiveProgress`))
      (for _array_element (`.Objectives_19_477E79AE4F539C86C339C682D01F5F05` (break `/Game/Game/Blueprints/Quests/S_QuestStage` _output_get_2))
        (`BlueprintMapLibrary.Map_Add` (`self.ObjectiveProgress`) (`.ID_9_57A6F44044E56A75E66920BB7B4CBE21` (break `/Game/Game/Blueprints/Quests/S_QuestObjective` _array_element)))))))

(fn `ObjectiveComplete`
  (params (ID :type String))
  (returns (Return :type Boolean))
  (`self.AllObjectivesComplete`)
  (return (>= (`BlueprintMapLibrary.Map_Find` (`self.ObjectiveProgress`) ID) (`.Quantity_12_E82C91294D60ACD3A26E7CB866C7DD17` (break `/Game/Game/Blueprints/Quests/S_QuestObjective` (`self.GetObjectiveDataByID` ID))))))

(fn `UserConstructionScript`)