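; BP_TurnSpawnerOn is a script Blueprint that spawns a group of five enemies at a hardcoded world location.
; RunScript finds the BP_EnemyGroupDirector and, if valid, calls SpawnGroup, then uses the result to look up the new group's members.
; Each member gets the "KLL_enemy" objective ID.
; The parent RunScript is called inside that loop, so it runs once per member rather than once overall.
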(fn `RunScript`
  (bind _returnvalue (`GameplayStatics.GetActorOfClass` "/Game/Game/Blueprints/Enemy/BP_EnemyGroupDirector.BP_EnemyGroupDirector_C"))
  (`/Engine/EditorBlueprintResources/StandardMacros.IsValid` _returnvalue
    (:`Is Valid`
      (bind _groupid (`/Game/Game/Blueprints/Enemy/BP_EnemyGroupDirector.SpawnGroup` _returnvalue (`KismetMathLibrary.MakeVector` 11240.0 14615.0 150.0) 5))
      (for _array_element (`.Members_6_10290FF94D5B363314413F8ACE398828` (break `/Game/Game/Blueprints/Enemy/S_EnemyGroup` (`|GetArrayItem` (`/Game/Game/Blueprints/Enemy/BP_EnemyGroupDirector.Groups` _returnvalue) _groupid)))
        (set `/Game/Game/Blueprints/Enemy/BP_Enemy.ObjectiveID` "KLL_enemy" _array_element)
        (`parent.RunScript`)))))

(fn `UserConstructionScript`
  (`parent.UserConstructionScript`))